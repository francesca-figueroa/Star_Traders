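; Star actor for Star Traders that shows a random zero to three orbiting planets and acts as a clickable trade point.
; On BeginPlay, chained count checks start a timeline per planet, moving it on a circle of increasing radius via sine and cosine, and hide unused planets.
; Clicking the star while the game mode's TestInventory is positive trades two units of it for one TestInventory2.
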(event EventBeginPlay
  (Variables|Default|SetnumberPlanets (Math|Random|RandomIntegerinRange 0 3))
  (Math|Integer|CompareInt (Variables|Default|GetnumberPlanets) 1
    (:>
      (bind _degrees (Timeline|Timeline_0 Play)
        (:Update
          (Transformation|SetRelativeLocation (Variables|Default|GetPlanet) (Math|Vector|MakeVector (* (Math|Trig|Cos(Degrees) _degrees) 2.4e+02) (* (Math|Trig|Sin(Degrees) _degrees) 2.4e+02) 0.0) false false)
          (Math|Integer|CompareInt (Variables|Default|GetnumberPlanets) 2
            (:>
              (bind _degrees_2 (Timeline|Timeline_1 Play)
                (:Update
                  (Transformation|SetRelativeLocation (Variables|Default|GetPlanet2) (Math|Vector|MakeVector (* (Math|Trig|Cos(Degrees) _degrees_2) 3.6e+02) (* (Math|Trig|Sin(Degrees) _degrees_2) 3.6e+02) 0.0) false false)
                  (Math|Integer|CompareInt (Variables|Default|GetnumberPlanets) 3
                    (:>
                      (bind _degrees_3 (Timeline|Timeline_2 Play)
                        (:Update
                          (Transformation|SetRelativeLocation (Variables|Default|GetPlanet3) (Math|Vector|MakeVector (* (Math|Trig|Cos(Degrees) _degrees_3) 4.8e+02) (* (Math|Trig|Sin(Degrees) _degrees_3) 4.8e+02) 0.0) false false)
                          (Input|EnableInput (Game|GetPlayerController 0) :!label _label))))
                    (:==
                      (Timeline|Timeline_2 Play))
                    (:<
                      (Rendering|SetVisibility (Variables|Default|GetPlanet3) false false :!label _label_2)
                      (goto _label))))))
            (:==
              (Timeline|Timeline_1 Play))
            (:<
              (Rendering|SetVisibility (Variables|Default|GetPlanet2) false false :!label _label_3)
              (goto _label_2))))))
    (:==
      (Timeline|Timeline_0 Play))
    (:<
      (Rendering|SetVisibility (Variables|Default|GetPlanet) false false)
      (goto _label_3))))

(event Collision|EventActorBeginOverlap
  (params (OtherActor :type Actor%20Object%20Reference)))

(event EventTick
  (params (DeltaSeconds :type Float%20%28single-precision%29)))

(event MouseInput|EventActorOnClicked
  (bind _asstar_traders_game_mode (Utilities|Casting|CastToStar_Traders_GameMode (Game|GetGameMode)))
  (Math|Integer|CompareInt (Variables|/Game/Star_Traders_Resorces/Blueprints/Star_Traders_GameMode.Star_Traders_GameMode_C|GettestInventory _asstar_traders_game_mode) 0
    (:>
      (Variables|/Game/Star_Traders_Resorces/Blueprints/Star_Traders_GameMode.Star_Traders_GameMode_C|SettestInventory _asstar_traders_game_mode (- (Variables|/Game/Star_Traders_Resorces/Blueprints/Star_Traders_GameMode.Star_Traders_GameMode_C|GettestInventory _asstar_traders_game_mode) 2))
      (Variables|/Game/Star_Traders_Resorces/Blueprints/Star_Traders_GameMode.Star_Traders_GameMode_C|SettestInventory2 _asstar_traders_game_mode (+ (Variables|/Game/Star_Traders_Resorces/Blueprints/Star_Traders_GameMode.Star_Traders_GameMode_C|GettestInventory2 _asstar_traders_game_mode) 1)))))

(fn ConstructionScript)