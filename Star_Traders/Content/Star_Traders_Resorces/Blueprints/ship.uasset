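; Ship actor for Star Traders that runs a test inventory exchange stored on the game mode.
; It enables input from the first player controller on BeginPlay and responds to any left mouse button release, with no check for what was clicked.
; While the game mode's TestInventory2 is above zero, each release converts one unit of it into three of TestInventory.
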(event EventBeginPlay
  (Input|EnableInput (Game|GetPlayerController 0)))

(event EventActorBeginOverlap
  (params (OtherActor :type Actor%20Object%20Reference)))

(event EventTick
  (params (DeltaSeconds :type Float%20%28single-precision%29)))

(event Input|MouseEvents|LeftMouseButton
  (params (Key :type Key%20Structure :default "AnyKey"))
  (:Released
    (bind _asstar_traders_game_mode (Utilities|Casting|CastToStar_Traders_GameMode (Game|GetGameMode)))
    (Math|Integer|CompareInt (Variables|/Game/Star_Traders_Resorces/Blueprints/Star_Traders_GameMode.Star_Traders_GameMode_C|GettestInventory2 _asstar_traders_game_mode) 0
      (:>
        (Variables|/Game/Star_Traders_Resorces/Blueprints/Star_Traders_GameMode.Star_Traders_GameMode_C|SettestInventory _asstar_traders_game_mode (+ (Variables|/Game/Star_Traders_Resorces/Blueprints/Star_Traders_GameMode.Star_Traders_GameMode_C|GettestInventory _asstar_traders_game_mode) 3))
        (Variables|/Game/Star_Traders_Resorces/Blueprints/Star_Traders_GameMode.Star_Traders_GameMode_C|SettestInventory2 _asstar_traders_game_mode (- (Variables|/Game/Star_Traders_Resorces/Blueprints/Star_Traders_GameMode.Star_Traders_GameMode_C|GettestInventory2 _asstar_traders_game_mode) 1))))))

(fn ConstructionScript)