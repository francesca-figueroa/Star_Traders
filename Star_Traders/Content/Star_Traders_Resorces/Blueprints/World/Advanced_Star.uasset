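; Star system actor for a space trading game that randomizes its economy, sun and orbiting planets on BeginPlay.
; It rolls a weighted system type (Farm, Mine, Industrial, Science, City), then randomly keeps matching spawn items as its means of production.
; It spawns randomly scaled and textured sphere planets at runtime.
; A Timeline moves them on circular orbits using sine and cosine, with per-index radius and speed.
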(event EventBeginPlay
  (bind _returnvalue (Math|Random|RandomIntegerinRange 1 6))
  (bind _items (CallFunction|GetItemsWorldSpawn))
  (Variables|Default|SetInvintory _items)
  (bind _type (CallFunction|SetStarType))
  (Variables|Default|SetSystemType _type)
  (bind _itemsonplanet (CallFunction|GetItemsbyType (Variables|Default|GetInvintory) (Variables|Default|GetSystemType)))
  (Utilities|Array|Clear (Variables|Default|GetMeans%20of%20Producion))
  (for _array_element _itemsonplanet
    (Math|Integer|CompareInt (Math|Random|RandomIntegerinRange 0 100) 40
      (:>
        _)
      (:==
        _))
    (Utilities|Array|Add (Variables|Default|GetMeans%20of%20Producion) _array_element))
  (CallFunction|SetRandomSunMaterial)
  (Variables|Default|SetnumberPlanets _returnvalue)
  (bind _list_of_planets (CallFunction|AddPlanets _returnvalue))
  (Variables|Default|SetPlanets%20Around%20Star _list_of_planets)
  (bind _degrees (Timeline|Timeline_0 Play)
    (:Update
      (for (_array_element_2 _array_index) (Variables|Default|GetPlanets%20Around%20Star)
        (Transformation|SetRelativeLocation _array_element_2 (Math|Vector|MakeVector (* (Math|Trig|Cos(Degrees) (* (Utilities|Array|Get(acopy) (Variables|Default|GetOrbit%20Speeds) _array_index) _degrees)) (Math|Conversions|ToFloat(Integer) (+ (* _array_index 30) 40))) (* (Math|Trig|Sin(Degrees) (* (Utilities|Array|Get(acopy) (Variables|Default|GetOrbit%20Speeds) _array_index) _degrees)) (Math|Conversions|ToFloat(Integer) (+ (* _array_index 30) 40))) (/ (.Z (Math|Vector|BreakVector (Variables|/Script/Engine.SceneComponent|GetRelativeScale3D _array_element_2))) -1.0)) false false)))))

(event Collision|EventActorBeginOverlap
  (params (OtherActor :type Actor%20Object%20Reference)))

(event EventTick
  (params (DeltaSeconds :type Float%20%28single-precision%29)))

(fn ConstructionScript)

(fn AddPlanets
  (params (Number%20of%20planets :type Integer))
  (for _index (range 0 Number%20of%20planets)
    (bind _returnvalue (AddComponent|AddStaticMeshComponent false))
    (Components|StaticMesh|SetStaticMesh _returnvalue "/Game/StarterContent/Shapes/Shape_Sphere.Shape_Sphere")
    (CallFunction|RandomPlanetMaterial _returnvalue)
    (Transformation|SetRelativeScale3D _returnvalue (Math|Vector|MakeVector (Math|Float|Clamp(Float) (/ (Math|Random|RandomFloatinRange 0.0 (Math|Conversions|ToFloat(Integer) _index)) 1e+01) 0.1 0.2) (Math|Float|Clamp(Float) (/ (Math|Random|RandomFloatinRange 0.0 (Math|Conversions|ToFloat(Integer) _index)) 1e+01) 0.1 0.2) (Math|Float|Clamp(Float) (/ (Math|Random|RandomFloatinRange 0.0 (Math|Conversions|ToFloat(Integer) _index)) 1e+01) 0.1 0.2)))
    (Utilities|Array|Add (LocalVariables|GetPlanets) _returnvalue))
  (return (LocalVariables|GetPlanets)))

(fn RandomPlanetMaterial
  (params (Planet :type Mesh%20Component%20Object%20Reference%20%28by%20ref%29))
  (switch int (Math|Random|RandomIntegerinRange 0 15)
    (:Default
      (Rendering|Material|SetMaterial Planet 0 "/Game/Star_Traders_Resorces/Materials/Desert.Desert" :!label _label))
    (:0
      (goto _label))
    (:1
      (Rendering|Material|SetMaterial Planet 0 "/Game/Star_Traders_Resorces/Materials/Grass.Grass"))
    (:2
      (Rendering|Material|SetMaterial Planet 0 "/Game/Star_Traders_Resorces/Materials/Ice_01.Ice_01"))
    (:3
      (Rendering|Material|SetMaterial Planet 0 "/Game/Star_Traders_Resorces/Materials/Mountain.Mountain"))
    (:4
      (Rendering|Material|SetMaterial Planet 0 "/Game/Star_Traders_Resorces/Materials/Mountain_02.Mountain_02"))
    (:5
      (Rendering|Material|SetMaterial Planet 0 "/Game/Star_Traders_Resorces/Materials/Neptune.Neptune"))
    (:6
      (Rendering|Material|SetMaterial Planet 0 "/Game/Star_Traders_Resorces/Materials/Rock_01.Rock_01"))
    (:7
      (Rendering|Material|SetMaterial Planet 0 "/Game/Star_Traders_Resorces/Materials/Rock_02.Rock_02"))
    (:8
      (Rendering|Material|SetMaterial Planet 0 "/Game/Star_Traders_Resorces/Materials/Rock_03.Rock_03"))
    (:9
      (Rendering|Material|SetMaterial Planet 0 "/Game/Star_Traders_Resorces/Materials/Rock_04.Rock_04"))
    (:10
      (Rendering|Material|SetMaterial Planet 0 "/Game/Star_Traders_Resorces/Materials/Sand.Sand"))
    (:11
      (Rendering|Material|SetMaterial Planet 0 "/Game/Star_Traders_Resorces/Materials/Snow.Snow"))
    (:12
      (Rendering|Material|SetMaterial Planet 0 "/Game/Star_Traders_Resorces/Materials/Terrain.Terrain"))
    (:13
      (Rendering|Material|SetMaterial Planet 0 "/Game/Star_Traders_Resorces/Materials/Water.Water"))
    (:14
      (Rendering|Material|SetMaterial Planet 0 "/Game/Star_Traders_Resorces/Materials/Water+Clouds.Water+Clouds"))))

(fn SetRandomSunMaterial
  (bind _sun (Variables|Default|GetSun))
  (switch int (Math|Random|RandomIntegerinRange 0 4)
    (:Default
      (Rendering|Material|SetMaterial _sun 0 "/Game/Star_Traders_Resorces/Materials/StarTest0.StarTest0" :!label _label))
    (:0
      (goto _label))
    (:1
      (Rendering|Material|SetMaterial _sun 0 "/Game/Star_Traders_Resorces/Materials/Sun_01.Sun_01"))
    (:2
      (Rendering|Material|SetMaterial _sun 0 "/Game/Star_Traders_Resorces/Materials/Sun_02.Sun_02"))
    (:3
      (Rendering|Material|SetMaterial _sun 0 "/Game/Star_Traders_Resorces/Materials/Sun_03.Sun_03"))
    (:4
      (Rendering|Material|SetMaterial _sun 0 "/Game/Star_Traders_Resorces/Materials/Sun_04.Sun_04"))))

(fn SetStarType
  (switch int (Math|Random|RandomIntegerinRange 0 16)
    (:Default
      (return "ERROR"))
    (:0
      _)
    (:1
      _)
    (:2
      _)
    (:3
      _)
    (:4
      (return "Mine"))
    (:5
      (return "Mine"))
    (:6
      (return "Mine"))
    (:7
      (return "Mine"))
    (:8
      (return "Industrial"))
    (:9
      (return "Industrial"))
    (:10
      (return "Industrial"))
    (:11
      (return "Science"))
    (:12
      (return "Science"))
    (:13
      (return "Science"))
    (:14
      (return "City"))
    (:15
      (return "City"))
    (:16
      (return "City")))
  (return "Farm"))