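; HexTile is a world tile actor that stores integer X and Y grid coordinates.
; Functions set the coordinate pair and return it as a vector with zero Z.
; Hovering the cursor over its Cube component prints the coordinates, and a mouse release on the actor prints a default string, which appears to be debug feedback.
; Begin play, tick and cursor exit contain no logic.
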(event OnBeginCursorOver(Cube)
  (params (TouchedComponent :type Primitive%20Component%20Object%20Reference))
  (Development|PrintString (Utilities|String|BuildString(Integer) (Utilities|String|ToString(Integer) (Variables|Default|GetX)) "," (Variables|Default|GetY))))

(event OnEndCursorOver(Cube)
  (params (TouchedComponent :type Primitive%20Component%20Object%20Reference)))

(event EventBeginPlay)

(event EventActorBeginOverlap
  (params (OtherActor :type Actor%20Object%20Reference)))

(event EventTick
  (params (DeltaSeconds :type Float%20%28single-precision%29)))

(event EventBeginPlay)

(event EventActorOnReleased
  (Development|PrintString "Hello"))

(fn ConstructionScript)

(fn HexTileSetXSetY
  (params (X :type Integer) (Y :type Integer))
  (Variables|Default|SetX X)
  (Variables|Default|SetY Y))

(fn HexTileGetCords
  (return (Math|Vector|MakeVector (Math|Conversions|ToFloat(Integer) (Variables|Default|GetX)) (Math|Conversions|ToFloat(Integer) (Variables|Default|GetY)) 0.0)))