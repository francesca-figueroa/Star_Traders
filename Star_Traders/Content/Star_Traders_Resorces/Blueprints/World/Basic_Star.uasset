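; Basic_Star is a world actor for a star with an orbiting planet and a click-driven test inventory exchange.
; On BeginPlay a timeline supplies degrees, and sine and cosine place the Planet component on a fixed-radius horizontal circle, with input re-enabled every update.
; Clicking the actor casts to Star_Traders_GameMode and, if TestInventory is above zero, subtracts two from it and adds one to TestInventory2.
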(event EventBeginPlay
  (bind _degrees (Timeline|Timeline_0 Play)
    (:Update
      (Transformation|SetRelativeLocation (Variables|Default|GetPlanet) (Math|Vector|MakeVector (* (Math|Trig|Cos(Degrees) _degrees) 2.4e+02) (* (Math|Trig|Sin(Degrees) _degrees) 2.4e+02) 0.0) false false)
      (Input|EnableInput (Game|GetPlayerController 0)))))

(event EventActorBeginOverlap
  (params (OtherActor :type Actor%20Object%20Reference)))

(event EventTick
  (params (DeltaSeconds :type Float%20%28single-precision%29)))

(event MouseInput|EventActorOnClicked
  (bind _asstar_traders_game_mode (Utilities|Casting|CastToStar_Traders_GameMode (Game|GetGameMode)))
  (Math|Integer|CompareInt (Variables|/Game/Star_Traders_Resorces/Blueprints/Star_Traders_GameMode.Star_Traders_GameMode_C|GettestInventory _asstar_traders_game_mode) 0
    (:>
      (Variables|/Game/Star_Traders_Resorces/Blueprints/Star_Traders_GameMode.Star_Traders_GameMode_C|SettestInventory _asstar_traders_game_mode (- (Variables|/Game/Star_Traders_Resorces/Blueprints/Star_Traders_GameMode.Star_Traders_GameMode_C|GettestInventory _asstar_traders_game_mode) 2))
      (Variables|/Game/Star_Traders_Resorces/Blueprints/Star_Traders_GameMode.Star_Traders_GameMode_C|SettestInventory2 _asstar_traders_game_mode (+ (Variables|/Game/Star_Traders_Resorces/Blueprints/Star_Traders_GameMode.Star_Traders_GameMode_C|GettestInventory2 _asstar_traders_game_mode) 1)))))

(fn ConstructionScript)