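; Star Traders game mode that generates the hex-tile star map when play begins.
; SpawnTiles lays HexTile actors in a grid with odd rows shifted sideways and gives each tile its grid coordinates.
; A random roll against a star density decides whether a scaled-down Advanced_Star spawns above each tile, which then stores a reference to it.
; An unconnected item lookup and print through PlayerCamera never runs.
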(event EventBeginPlay
  (CallFunction|SpawnTiles 9 9 20))

(event EventTick
  (params (DeltaSeconds :type Float%20%28single-precision%29)))

(fn ConstructionScript)

(fn SpawnTiles
  (params (y1 :type Integer) (x1 :type Integer) (Star%20Density :type Integer))
  (for _index (range 0 y1)
    (for _index_2 (range 0 x1)
      (bind _output_get (LocalVariables|SetSpawnOffSet (Math|Vector|MakeVector (Math|Conversions|ToFloat(Integer) (+ (* _index_2 205) (* (Math|Integer|%(Integer) _index 2) 95))) (Math|Conversions|ToFloat(Integer) (* _index 174)) 0.0)))
      (bind _returnvalue (Game|SpawnActorfromClass "/Game/Star_Traders_Resorces/Blueprints/World/HexTile.HexTile_C" (Math|Conversions|ToTransform(Vector) _output_get) "AlwaysSpawn" 0 0))
      (Default|HexTileSetXSetY _returnvalue _index_2 _index)
      (Math|Integer|CompareInt (Math|Random|RandomIntegerinRange 0 100) Star%20Density
        (:<
          (bind _returnvalue_2 (Game|SpawnActorfromClass "/Game/Star_Traders_Resorces/Blueprints/World/Advanced_Star.Advanced_Star_C" (Math|Transform|MakeTransform (Math|Vector|MakeVector (Math|Conversions|ToFloat(Integer) (+ (* _index_2 205) (* (Math|Integer|%(Integer) _index 2) 95))) (Math|Conversions|ToFloat(Integer) (* _index 174)) 64.0) "0, 0, 0" "0.500000,0.500000,0.500000") "Undefined" 0 0))
          (Variables|/Game/Star_Traders_Resorces/Blueprints/World/HexTile.HexTile_C|SetTilesStar _returnvalue _returnvalue_2))))))